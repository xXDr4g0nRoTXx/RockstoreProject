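; Fetch quest pickup, apparently a wrench, that the player collects with the Interaction input while in range.
; Box overlap by the third-person character enables input, shows the ItemHere prompt and opens a Gate; leaving reverses all three.
; Pressing Interaction increments the character's Score, plays a sound, briefly shows ShowWrench, swaps it for ShowWrenchForever, then destroys the actor.
; ToggleHide and ShowItems are present but never run.
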(event OnComponentBeginOverlap(Box)
  (params (OverlappedComponent :type Primitive%20Component%20Object%20Reference) (OtherActor :type Actor%20Object%20Reference) (OtherComp :type Primitive%20Component%20Object%20Reference) (OtherBodyIndex :type Integer) (bFromSweep :type Boolean) (SweepResult :type Hit%20Result%20Structure%20%28by%20ref%29))
  (bind _asbp_third_person_character (Utilities|Casting|CastToBP_ThirdPersonCharacter OtherActor))
  (Variables|Default|SetThirdPersonRef _asbp_third_person_character)
  (Input|EnableInput (Game|GetPlayerController 0))
  (bind _returnvalue (UserInterface|CreateWidget "/Game/Blueprint/Text/ItemHere.ItemHere_C"))
  (UserInterface|Viewport|AddtoViewport _returnvalue 0)
  (Utilities|FlowControl|Gate true) ; enters at Open
)

(event OnComponentEndOverlap(Box)
  (params (OverlappedComponent :type Primitive%20Component%20Object%20Reference) (OtherActor :type Actor%20Object%20Reference) (OtherComp :type Primitive%20Component%20Object%20Reference) (OtherBodyIndex :type Integer))
  (bind _asbp_third_person_character (Utilities|Casting|CastToBP_ThirdPersonCharacter OtherActor))
  (Variables|Default|SetThirdPersonRef _asbp_third_person_character)
  (Input|DisableInput (Game|GetPlayerController 0))
  (bind _foundwidgets (Widget|GetAllWidgetsOfClass "/Game/Blueprint/Text/ItemHere.ItemHere_C" true))
  (Widget|RemovefromParent _foundwidgets)
  (Utilities|FlowControl|Gate true) ; enters at Close
)

(event Input|ActionEvents|InputActionInteraction
  (params (Key :type Key%20Structure :default "None"))
  (:Pressed
    (Utilities|FlowControl|Gate true
      (:Exit
        (bind _asbp_third_person_character (Utilities|Casting|CastToBP_ThirdPersonCharacter (Game|GetPlayerCharacter 0)))
        (Variables|/Game/ThirdPerson/Blueprints/BP_ThirdPersonCharacter.BP_ThirdPersonCharacter_C|SetScore _asbp_third_person_character (+ (Variables|/Game/ThirdPerson/Blueprints/BP_ThirdPersonCharacter.BP_ThirdPersonCharacter_C|GetScore _asbp_third_person_character) 1))
        (Audio|PlaySound2D "/Game/ThirdPerson/A_fairy_dust_1__1_.A_fairy_dust_1__1_" 1.0 1.0 0.0 0 0)
        (bind _foundwidgets (Widget|GetAllWidgetsOfClass "/Game/Blueprint/Text/ItemHere.ItemHere_C" true))
        (Widget|RemovefromParent _foundwidgets)
        (bind _returnvalue (UserInterface|CreateWidget "/Game/PNG/Items/ShowWrench.ShowWrench_C"))
        (UserInterface|Viewport|AddtoViewport _returnvalue 0)
        (Utilities|FlowControl|Delay 1.0)
        (bind _foundwidgets_2 (Widget|GetAllWidgetsOfClass "/Game/PNG/Items/ShowWrench.ShowWrench_C" true))
        (Widget|RemovefromParent _foundwidgets_2)
        (bind _returnvalue_2 (UserInterface|CreateWidget "/Game/PNG/Items/ShowWrenchForever.ShowWrenchForever_C"))
        (UserInterface|Viewport|AddtoViewport _returnvalue_2 0)
        (Actor|DestroyActor)))))

(fn ConstructionScript)

(fn ToggleHide
  (bind _jones_ref (Variables|Default|GetJones%20Ref))
  (if (Variables|Default|GetIsHiding?)
    (Variables|Default|SetIsHiding? false)
    (Rendering|SetActorHiddenInGame _jones_ref false)
    (Collision|SetActorEnableCollision _jones_ref true)
    (else
      (Variables|Default|SetIsHiding? true)
      (Rendering|SetActorHiddenInGame _jones_ref true)
      (Collision|SetActorEnableCollision _jones_ref false))))

(fn ShowItems
  (bind _returnvalue (UserInterface|CreateWidget "/Game/PNG/Items/ShowWrench.ShowWrench_C"))
  (UserInterface|Viewport|AddtoViewport _returnvalue 0)
  (Class|SubmixEffectDelayStatics|SetDelayLength (Variables|Default|GetDelay%20Settings) 2.0)
  (bind _foundwidgets (Widget|GetAllWidgetsOfClass "/Game/Blueprint/Text/ItemHere.ItemHere_C" true))
  (Widget|RemovefromParent _foundwidgets))