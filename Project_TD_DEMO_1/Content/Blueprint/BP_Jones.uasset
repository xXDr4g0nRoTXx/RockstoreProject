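; Paper2D side-scrolling player character Jones, with horizontal movement, sprinting, health and a death screen.
; Tick swaps idle and run flipbooks by velocity, flips facing through controller yaw and plays footstep sounds on two animation frames.
; Sprinting changes walk speed and starts self-calling delayed events that drain or regenerate stamina, stopping the sprint at zero.
; BeginPlay fades the camera and adds the score widget; an M key self-damages.
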(event Custom|Update%20Animation
  (Sprite|SetFlipbook (Variables|Default|GetSprite) (select (> (Math|Vector|VectorLength (Variables|/Script/Engine.MovementComponent|GetVelocity (Variables|Character|GetCharacterMovement))) 0.0) "/Game/Jones/RunRight/Jones_Run.Jones_Run" "/Game/Jones/Jones_Idle.Jones_Idle")))

(event Custom|Update%20Rotation
  (Utilities|IsValid (Pawn|GetController)
    (:Is%20Valid
      (Math|Float|CompareFloat (.X (Math|Vector|BreakVector (Variables|/Script/Engine.MovementComponent|GetVelocity (Variables|Character|GetCharacterMovement)))) 0.0
        (:>
          (Pawn|SetControlRotation (Pawn|GetController) (Math|Rotator|MakeRotator 0.0 0.0 0.0)))
        (:<
          (Pawn|SetControlRotation (Pawn|GetController) (Math|Rotator|MakeRotator 0.0 0.0 1.8e+02)))))))

(event Custom|GainStamina
  (bind _output_get (Variables|Default|SetStamina (Math|Integer|Clamp(Integer) (+ (Variables|Default|GetStamina) 2) 0 (Variables|Default|GetMax%20stamina))))
  (if (not (== _output_get (Variables|Default|GetMax%20stamina)))
    (if (not (Variables|Default|GetIsSprinting?))
      (Utilities|FlowControl|Delay 0.1)
      (CallFunction|GainStamina))))

(event Custom|DrainStamina
  (bind _output_get (Variables|Default|SetStamina (Math|Integer|Clamp(Integer) (- (Variables|Default|GetStamina) 5) 0 (Variables|Default|GetMax%20stamina))))
  (if (== _output_get 0)
    (CallFunction|StopSprinting)
    (elif (Variables|Default|GetIsSprinting?)
      (Utilities|FlowControl|Delay 0.1)
      (CallFunction|DrainStamina))))

(event EventBeginPlay
  (CameraFades|StartCameraFade :self (Game|GetPlayerCameraManager 0) :FromAlpha 1.0 :Duration 3.0 :bHoldWhenFinished true)
  (bind _returnvalue (UserInterface|CreateWidget "/Game/Blueprint/ScoreBP/Score.Score_C"))
  (UserInterface|Viewport|AddtoViewport _returnvalue 0))

(event Game|Damage|EventAnyDamage
  (params (Damage :type Float%20%28single-precision%29) (DamageType :type Damage%20Type%20Object%20Reference) (InstigatedBy :type Controller%20Object%20Reference) (DamageCauser :type Actor%20Object%20Reference))
  (Variables|Default|SetHeatlh (- (Variables|Default|GetHeatlh) Damage))
  (if (<= (Variables|Default|GetHeatlh) 0.0)
    (Development|PrintString "Dead")
    (bind _returnvalue (UserInterface|CreateWidget "/Game/Blueprint/UI/DeathScreen.DeathScreen_C"))
    (UserInterface|Viewport|AddtoViewport _returnvalue 0)
    (else
      (Development|PrintString (Utilities|String|ToString(Float) (Variables|Default|GetHeatlh))))))

(event EventTick
  (params (DeltaSeconds :type Float%20%28single-precision%29))
  (bind _sprite (Variables|Default|GetSprite))
  (bind _returnvalue (Class|PaperFlipbookComponent|GetPlaybackPositioninFrames _sprite))
  (CallFunction|UpdateAnimation)
  (CallFunction|UpdateRotation)
  (if (or (== _returnvalue 1) (== _returnvalue 18))
    (Audio|PlaySound2D "/Game/Sound/Concrete_Step_Cue.Concrete_Step_Cue" 1.0 1.0 0.0 0 0)))

(event Input|ActionEvents|InputActionSprint
  (params (Key :type Key%20Structure))
  (:Pressed
    (CallFunction|StartSprinting))
  (:Released
    (CallFunction|StopSprinting)))

(event Input|AxisEvents|InputAxisMoveRight
  (params (AxisValue :type Float%20%28single-precision%29))
  (Pawn|Input|AddMovementInput "0.500000,0.000000,0.000000" AxisValue false))

(event Input|KeyboardEvents|M
  (params (Key :type Key%20Structure))
  (:Pressed
    (Game|Damage|ApplyDamage self 1e+01 0 0)))

(fn ConstructionScript)

(fn StartSprinting
  (Variables|/Script/Engine.CharacterMovementComponent|SetMaxWalkSpeed (Variables|Character|GetCharacterMovement) 7e+02)
  (Variables|Default|SetIsSprinting? true)
  (CallFunction|DrainStamina))

(fn StopSprinting
  (Variables|/Script/Engine.CharacterMovementComponent|SetMaxWalkSpeed (Variables|Character|GetCharacterMovement) 4e+02)
  (Variables|Default|SetIsSprinting? false)
  (CallFunction|GainStamina))